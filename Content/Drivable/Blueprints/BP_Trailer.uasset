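; Drivable trailer that can be hitched to and unhitched from a BP_Car.
; While a car overlaps the Trigger, a Delay loop compares its Dock position to the Trigger and shows TextDock when within tolerance.
; When docking is possible, Interact alternates between binding both meshes with a PhysicsConstraint plus slight trailer throttle, and breaking the constraint with zero throttle.
; Construction enlarges the mesh bounds.
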(event `self.Trigger.OnComponentBeginOverlap`
  (params (OverlappedComponent :type "PrimitiveComponent Object Reference") (OtherActor :type "Actor Object Reference") (OtherComp :type "PrimitiveComponent Object Reference") (OtherBodyIndex :type Integer) (bFromSweep :type Boolean) (SweepResult :type "HitResult Structure (by ref)"))
  (if (== (`GameplayStatics.GetObjectClass` OtherActor) "/Game/Drivable/Blueprints/BP_Car.BP_Car_C")
    (set `self.TryDock` true)
    (bind _asbp_car (cast `/Game/Drivable/Blueprints/BP_Car` OtherActor :!label _label))
    (bind _output_get (set `self.CanDock` (== (`SceneComponent.K2_GetComponentLocation` (`self.Trigger`)) (`SceneComponent.K2_GetComponentLocation` (`/Game/Drivable/Blueprints/BP_Car.Dock` _asbp_car)) :`ErrorTolerance` 100.0)))
    (`SceneComponent.SetVisibility` (`self.TextDock`) _output_get false)
    (`KismetSystemLibrary.Delay` 0.2)
    (if (`self.TryDock`)
      (goto _label))))

(event `/Game/Drivable/Blueprints/IBP_Interact.Interact`
  (params (Car :type "/Game/Drivable/Blueprints/BP_Car Object Reference"))
  (bind _vehiclemovementcomponent (`self.VehicleMovementComponent`))
  (bind _physicsconstraint (`self.PhysicsConstraint`))
  (if (`self.CanDock`)
    (`/Engine/EditorBlueprintResources/StandardMacros.FlipFlop`
      (:`A`
        (`ChaosVehicleMovementComponent.SetThrottleInput` _vehiclemovementcomponent 0.01)
        (`PhysicsConstraintComponent.SetConstrainedComponents` _physicsconstraint (`WheeledVehiclePawn.Mesh` Car) "Root" (`self.Mesh`) "Root")
        (set `self.TryDock` false))
      (:`B`
        (`ChaosVehicleMovementComponent.SetThrottleInput` _vehiclemovementcomponent 0.0)
        (`PhysicsConstraintComponent.BreakConstraint` _physicsconstraint)
        (set `self.TryDock` true)))
    (`SceneComponent.SetVisibility` (`self.TextDock`) (`self.TryDock`) false)))

(event `self.Trigger.OnComponentEndOverlap`
  (params (OverlappedComponent :type "PrimitiveComponent Object Reference") (OtherActor :type "Actor Object Reference") (OtherComp :type "PrimitiveComponent Object Reference") (OtherBodyIndex :type Integer))
  (if (== (`GameplayStatics.GetObjectClass` OtherActor) "/Game/Drivable/Blueprints/BP_Car.BP_Car_C")
    (cast `/Game/Drivable/Blueprints/BP_Car` OtherActor)
    (set `self.TryDock` false)
    (`SceneComponent.SetVisibility` (`self.TextDock`) false false)))

(fn `UserConstructionScript`
  (`PrimitiveComponent.SetBoundsScale` (`self.Mesh`) 5.0))